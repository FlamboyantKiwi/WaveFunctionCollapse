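; Generator actor that runs Wave Function Collapse over a tile grid and visualizes it on screen.
; On BeginPlay it registers goblin, human and ogre data assets as available tiles, initializes the grid and builds a WBP_WFCBoard widget.
; A timer, looping if auto-stepping, calls StepWfc, refreshing the board until completion clears it.
; ToggleAutoStep only flips its flag, leaving the running timer untouched.
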(event Custom|WFC%20Step
  (bind _returnvalue (Class|WfcGenerator|StepWfc))
  (if _returnvalue
    (Utilities|Time|ClearandInvalidateTimerbyHandle (Variables|Default|GetstepTimerHandle))
    (Development|PrintString "WFC Complete!")
    (else
      (Default|RefreshBoard (Variables|Default|GetBoard) (Variables|Default|GetGrid)))))

(event Custom|ToggleAutoStep
  (bind _output_get (Variables|Default|SetisAutoStepping (not (Variables|Default|GetisAutoStepping))))
  (if _output_get
    _))

(event EventBeginPlay
  (bind _gridsize (Variables|Default|GetGridSize))
  (CallFunction|AddDataTypes)
  (Class|WfcGenerator|InitializeGrid)
  (bind _returnvalue (UserInterface|CreateWidget "/Game/WFC/WBP_WFCBoard.WBP_WFCBoard_C"))
  (bind _output_get (Variables|Default|SetBoard _returnvalue))
  (UserInterface|Viewport|AddtoViewport _output_get 0)
  (Default|GenerateGrid (Variables|Default|GetBoard) (.x _gridsize) (.y _gridsize))
  (bind _returnvalue_2 (Utilities|Time|SetTimerbyEvent (delegate Custom|WFC%20Step) (Variables|Default|GetstepDelay) (Variables|Default|GetisAutoStepping)))
  (Variables|Default|SetstepTimerHandle _returnvalue_2))

(fn ConstructionScript)

(fn AddDataTypes
  (bind _availabletiles (Variables|Default|GetAvailableTiles))
  (Utilities|Array|Add _availabletiles "/Game/WFC/DataAssets/DA_Goblin.DA_Goblin")
  (Utilities|Array|Add _availabletiles "/Game/WFC/DataAssets/DA_Human.DA_Human")
  (Utilities|Array|Add _availabletiles "/Game/WFC/DataAssets/DA_Ogre.DA_Ogre"))